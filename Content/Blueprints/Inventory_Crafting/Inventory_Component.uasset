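; Inventory component that tracks item quantities in a map for the inventory and crafting system.
; AddToInventory adds to the stored count, clamps it between 0 and 99, and always reports success.
; QueryInventory returns the held count and whether the item exists in at least the requested quantity.
; RemoveFromInventory uses that query to subtract only when enough is held, leaving depleted items in the map at zero.
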(event EventBeginPlay)

(event EventTick
  (params (DeltaSeconds :type Float%20%28single-precision%29)))

(fn AddtoInventory
  (params (ItemToBeAdded :type BP%20Breakable%20Class%20Reference) (Quanitity :type Integer))
  (Utilities|Map|Add (Variables|Default|GetInventory) ItemToBeAdded (Math|Integer|Clamp(Integer) (+ Quanitity (.Value (Utilities|Map|Find (Variables|Default|GetInventory) ItemToBeAdded))) 0 99))
  (return true))

(fn QueryInventory
  (params (Item :type BP%20Breakable%20Class%20Reference) (Quantity :type Integer))
  (bind _inventory (Variables|Default|GetInventory))
  (bind (_value _returnvalue) (Utilities|Map|Find _inventory Item))
  (if (and (>= _value Quantity) _returnvalue)
    (return _value true)
    (else
      (return _value false))))

(fn RemovefromInventory
  (params (ItemToBeRemoved :type BP%20Breakable%20Class%20Reference) (Quantity :type Integer))
  (bind (_output_quantity _success) (CallFunction|QueryInventory ItemToBeRemoved Quantity))
  (if _success
    (Utilities|Map|Add (Variables|Default|GetInventory) ItemToBeRemoved (- _output_quantity Quantity))
    (return true)
    (else
      (return false))))