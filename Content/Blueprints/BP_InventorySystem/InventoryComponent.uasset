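; Inventory component that toggles the player's inventory window on the HUD.
; ToggleInventory creates the window widget with a reference to itself and adds it to the player controller's HUD canvas, auto-sized, center-anchored and placed at a Position variable.
; A valid stored window is removed and cleared instead, with input switching between UI-only and game-only and debug prints on each toggle.
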(event EventBeginPlay)

(event EventTick
  (params (DeltaSeconds :type Float%20%28single-precision%29)))

(fn ToggleInventory
  (Variables|Default|GetInventory_Window
    (:then
      (Widget|RemovefromParent (Variables|Default|GetInventory_Window))
      (Development|PrintString "Close")
      (Variables|Default|SetInventory_Window 0)
      (Input|SetInputModeGameOnly (Game|GetPlayerController 0)))
    (:else
      (bind _returnvalue (UserInterface|CreateWidget "/Game/Blueprints/BP_InventorySystem/InventoryUI/InventoryWindow.InventoryWindow_C" 0 self))
      (Development|PrintString "Open")
      (Variables|Default|SetInventory_Window _returnvalue)
      (bind _asmy_player_controller (Utilities|Casting|CastToMyPlayer_Controller (Game|GetPlayerController 0)))
      (bind _returnvalue_2 (Class|CanvasPanel|AddChildtoCanvas (Variables|/Game/Blueprints/BP_InventorySystem/InventoryUI/HUD.HUD_C|GetHud_Canvas (Variables|/Game/Blueprints/BP_InventorySystem/Player_Controller/MyPlayer_Controller.MyPlayer_Controller_C|GetHudWidget _asmy_player_controller)) (Variables|Default|GetInventory_Window)))
      (Class|CanvasPanelSlot|SetAutoSize _returnvalue_2 true)
      (Class|CanvasPanelSlot|SetAlignment _returnvalue_2 "(X=0.500000,Y=0.500000)")
      (Class|CanvasPanelSlot|SetAnchors _returnvalue_2 (Utilities|Struct|MakeAnchors "(X=0.500000,Y=0.500000)" "(X=0.500000,Y=0.500000)"))
      (Class|CanvasPanelSlot|SetPosition _returnvalue_2 (Variables|Default|GetPosition))
      (Input|SetInputModeUIOnly (Game|GetPlayerController 0) (Variables|Default|GetInventory_Window) "DoNotLock"))))