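; BP_Ground is a ground actor that damages BP_Breakable objects falling onto it.
; It arms itself after a short delay from BeginPlay, so earlier hits do no damage.
; Once armed, a hit from a breakable with enough downward velocity applies small-radius, full radial damage at the impact point.
; The same hit also gives the struck component an upward impulse.
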(event Collision|EventHit
  (params (MyComp :type Primitive%20Component%20Object%20Reference) (Other :type Actor%20Object%20Reference) (OtherComp :type Primitive%20Component%20Object%20Reference) (bSelfMoved :type Boolean) (HitLocation :type Vector :default "0, 0, 0") (HitNormal :type Vector :default "0, 0, 0") (NormalImpulse :type Vector :default "0, 0, 0") (Hit :type Hit%20Result%20Structure%20%28by%20ref%29))
  (if (Variables|Default|GetDamaging)
    (bind _asbp_breakable (Utilities|Casting|CastToBP_Breakable Other))
    (if (<= (.z (Transformation|GetVelocity _asbp_breakable)) -4e+01)
      (Game|Damage|ApplyRadialDamage 2e+02 HitLocation 2e+01 0 0 0 0 true "ECC_Visibility")
      (Physics|AddImpulse OtherComp "0, 0,50.000000" "None" false))))

(event EventBeginPlay
  (Utilities|FlowControl|Delay 3.0)
  (Variables|Default|SetDamaging true))

(fn ConstructionScript)