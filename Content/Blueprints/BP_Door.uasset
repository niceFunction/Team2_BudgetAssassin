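; BP_Door is a door that unlocks when a FirstPersonCharacter holding the door key overlaps its Box1 trigger.
; On that overlap it sets Opened and deactivates its NavModifier, removing that modifier's effect on navigation.
; BeginPlay caches the mesh's world transform, but the node that would set that transform is unconnected, so this graph never moves the mesh.
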(event OnComponentBeginOverlap(Box1)
  (params (OverlappedComponent :type Primitive%20Component%20Object%20Reference) (OtherActor :type Actor%20Object%20Reference) (OtherComp :type Primitive%20Component%20Object%20Reference) (OtherBodyIndex :type Integer) (bFromSweep :type Boolean) (SweepResult :type Hit%20Result%20Structure%20%28by%20ref%29))
  (bind _asfirst_person_character (Utilities|Casting|CastToFirstPersonCharacter OtherActor))
  (if (Variables|/Game/FirstPersonBP/Blueprints/FirstPersonCharacter.FirstPersonCharacter_C|GetHasDoorKey _asfirst_person_character)
    (Variables|Default|SetOpened true)
    (Components|Activation|Deactivate (Variables|Default|GetNavModifier))))

(event EventBeginPlay
  (|CallParentFunction)
  (Variables|Default|SetWorldTransform (Transformation|GetWorldTransform (Variables|Character|GetMesh))))

(event EventTick
  (params (DeltaSeconds :type Float%20%28single-precision%29))
  (|CallParentFunction DeltaSeconds))

(fn ConstructionScript
  (|CallParentFunction))