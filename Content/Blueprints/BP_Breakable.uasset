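; BP_Breakable is a physics prop that attaches to another actor, breaks off under damage, and can be grabbed or picked up into the inventory.
; Damage lowers Durability while AttachedTo is valid, detaching at zero; otherwise it passes to a random attached actor.
; Tick drives spring-like grabbing with distance-scaled impulses toward the player's Grabpoint, releasing past a force threshold.
; Detached inventory items without attached breakables become pickable; interacting adds them to inventory and destroys the actor.
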(event Custom|Asd
  (bind _self self)
  (bind _returnvalue (Transformation|GetVelocity _self))
  (bind _returnvalue_2 (Math|Vector|VectorLength _returnvalue))
  (Variables|Default|SetAverageVelocity (- (/ (Variables|Default|GetAverageVelocity) 2.2) 1e+01))
  (if (> _returnvalue_2 1.0)
    (Variables|Default|SetAverageVelocity (+ _returnvalue_2 (Variables|Default|GetAverageVelocity)))))

(event EventBeginPlay
  (Utilities|GetReferencetoPlayer)
  (Utilities|AttachThisObjecttoAttachto))

(event EventInteractwith
  (params (PlayerCharacter :type First%20Person%20Character%20Object%20Reference))
  (Development|PrintString "Picked Up" true true "(R=1.000000,G=0.000000,B=0.276783,A=1.000000)" 3.0)
  (Development|PrintString (Utilities|String|ToString(Text) (Variables|Default|GetName)) true true "(R=0.000000,G=0.660000,B=1.000000,A=1.000000)" 3.0)
  (Default|AddtoInventory (Variables|/Game/FirstPersonBP/Blueprints/FirstPersonCharacter.FirstPersonCharacter_C|GetInventory_Component PlayerCharacter) (Utilities|GetClass self) 1)
  (bind _asplayer_controller (Utilities|Casting|CastToPlayer_Controller (Game|GetPlayerController 0)))
  (Default|RefreshInventory (Variables|/Game/Blueprints/Inventory_Crafting/HeadsUpDisplay.HeadsUpDisplay_C|GetCraftingMenu (Variables|/Game/Blueprints/Inventory_Crafting/Player_Controller.Player_Controller_C|GetHeadsUpDisplay _asplayer_controller)))
  (Effects|SpawnEmitteratLocation "/Game/StarterContent/Particles/P_Explosion.P_Explosion" (Transformation|GetActorLocation) "0, 0, 0" "0.010000,0.010000,0.010000")
  (Actor|DestroyActor))

(event EventTick
  (params (DeltaSeconds :type Float%20%28single-precision%29))
  (CallFunction|Asd)
  (Utilities|GetGrabVariables)
  (bind _returnvalue (Utilities|GrabPhysics))
  (Utilities|GrabLimiter _returnvalue)
  (Utilities|AttachRefresh)
  (Utilities|SetasPickable))

(event Game|Damage|EventAnyDamage
  (params (Damage :type Float%20%28single-precision%29) (DamageType :type Damage%20Type%20Object%20Reference) (InstigatedBy :type Controller%20Object%20Reference) (DamageCauser :type Actor%20Object%20Reference))
  (Utilities|DealDamagetoOthes Damage
    (:Is%20Invalid
      (Utilities|PrintBrokenifTrue :!label _label)
      (Utilities|DetachfromEverything)
      (Utilities|SetasPickable))
    (:Is%20Valid
      (Utilities|DealDamagetoDurability Damage
        (:Broken
          (goto _label))
        (:Damaged
          (Utilities|PrintDamagedifTrue))))))

(fn ConstructionScript
  (Rendering|SetVisibility (Variables|Default|GetAnchorPointMesh) (Variables|GrabSystem|GetShowGrabSpot) false))