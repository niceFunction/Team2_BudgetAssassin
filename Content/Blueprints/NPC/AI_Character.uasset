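; AI-controlled NPC character that patrols between two target points, roams to random navigable points or chases the first-person player.
; AIState is read once at BeginPlay to start one self-repeating AIMoveTo loop; the see-pawn event is empty.
; Damage drains Health, and at zero the mesh becomes a ragdoll and IsDead stops the loops from restarting.
; A falling BP_Breakable hit triggers radial damage plus extra self-damage.
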(event OnSeePawn(PawnSensing)
  (params (Pawn :type Pawn%20Object%20Reference))
  ;[1 1 1] Change state
)

(event Custom|Roam
  ;[1 1 1] Roam
  (if (not (Variables|Default|GetIsDead))
    (AI|AIMoveTo self (.RandomLocation (Class|NavigationSystemV1|GetRandomPointinNavigableRadius (Transformation|GetActorLocation) 1.5e+03 0 0)) 0 5.0 false
      (:OnSuccess
        _)
      (:OnFail
        _))
    (Utilities|FlowControl|Delay 1.0)
    (CallFunction|Roam)))

(event Custom|Patrol
  ;[1 1 1] Patrol
  (if (not (Variables|Default|GetIsDead))
    (AI|AIMoveTo self "0, 0, 0" (Variables|Default|GetTargetPoint1) 5.0 false
      (:OnSuccess
        (Utilities|FlowControl|Delay 2.0)
        (AI|AIMoveTo self "0, 0, 0" (Variables|Default|GetTargetPoint2) 5.0 false
          (:OnSuccess
            (Utilities|FlowControl|Delay 2.2)
            (CallFunction|Patrol)))))))

(event Custom|Chase
  ;[1 1 1] Chase
  (if (not (Variables|Default|GetIsDead))
    (AI|AIMoveTo self (Transformation|GetActorLocation (Variables|Default|GetFirstPersonCharacter)) 0 1e+03 false
      (:then
        (Utilities|FlowControl|Delay 1.0)
        (CallFunction|Chase)))))

(event EventBeginPlay
  (Utilities|FlowControl|Sequence
    (:then_0
      (bind _outactors (Actor|GetAllActorsOfClass "/Game/FirstPersonBP/Blueprints/FirstPersonCharacter.FirstPersonCharacter_C"))
      (Variables|Default|SetFirstPersonCharacter (Utilities|Array|Get(acopy) _outactors)))
    (:then_1
      (switch Utilities|FlowControl|Switch|SwitchonEAIState (Variables|Default|GetAIState)
        (:NewEnumerator0
          (CallFunction|Patrol))
        (:NewEnumerator1
          (CallFunction|Roam))
        (:NewEnumerator2
          (CallFunction|Chase))))))

(event Game|Damage|EventAnyDamage
  (params (Damage :type Float%20%28single-precision%29) (DamageType :type Damage%20Type%20Object%20Reference) (InstigatedBy :type Controller%20Object%20Reference) (DamageCauser :type Actor%20Object%20Reference))
  (bind _mesh (Variables|Character|GetMesh))
  (Variables|Default|SetHealth (- (Variables|Default|GetHealth) Damage))
  (if (<= (Variables|Default|GetHealth) 0.0)
    (Collision|SetCollisionProfileName _mesh "Raggdoll" true :!class /Script/Engine.PrimitiveComponent)
    (Physics|SetSimulatePhysics _mesh true)
    (Audio|Components|Audio|Stop (Variables|Character|GetMesh))
    (Variables|Default|SetIsDead true)))

(event Collision|EventHit
  (params (MyComp :type Primitive%20Component%20Object%20Reference) (Other :type Actor%20Object%20Reference) (OtherComp :type Primitive%20Component%20Object%20Reference) (bSelfMoved :type Boolean) (HitLocation :type Vector :default "0, 0, 0") (HitNormal :type Vector :default "0, 0, 0") (NormalImpulse :type Vector :default "0, 0, 0") (Hit :type Hit%20Result%20Structure%20%28by%20ref%29))
  (bind _asbp_breakable (Utilities|Casting|CastToBP_Breakable Other))
  (if (<= (.z (Transformation|GetVelocity _asbp_breakable)) -1e+01)
    (bind _returnvalue (Game|Damage|ApplyRadialDamage 2e+02 HitLocation 2e+02 0 0 0 0 true "ECC_Visibility"))
    (if _returnvalue
      (Game|Damage|ApplyDamage self 1e+02 0 0))))

(fn ConstructionScript)